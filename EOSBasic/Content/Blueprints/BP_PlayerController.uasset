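; Player controller that serves as a manual test harness for an Epic Online Services (EOS) integration.
; Input actions initialize or shut down the SDK through the EOS manager and drive Metrics setup and player sessions, printing each result on screen.
; Login and Logout only print a warning about Epic Store and C++ requirements.
; The authentication binding, DevTool login and manual update code are left unconnected.
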(event `self.ReceiveTick`
  (params (DeltaSeconds :type "Float (single-precision)")))

(event `InputAction|StartEOS`
  (params (Key :type "Key Structure"))
  ;[1 1 1] Attempt to Initialize the EOS SDK.  You might put this in some of your own code that performs start-up tasks.
  (:`Released`
    (bind (_activeeosmanager _returnvalue) (`EOSManager.RequestEOSManager`))
    (if _returnvalue
      (bind _returnvalue_2 (`EOSManager.InitEOS` _activeeosmanager))
      (`KismetSystemLibrary.PrintString` (`KismetStringLibrary.Concat_StrStr` "Init Success?: " (`|GetEnumeratorNameAsString` _returnvalue_2)) true true (struct :`G` 0.66 :`B` 1.0 :`A` 1.0) 10.0))))

(event `InputAction|ShutdownEOS`
  (params (Key :type "Key Structure"))
  ;[1 1 1] Attempt to Shutdown the EOS SDK.  You might put this in your Game Instance's "Event Shutdown" so that this can occur before anything else is torn down, destroyed or disconnected.
  (:`Released`
    (bind (_activeeosmanager _returnvalue) (`EOSManager.RequestEOSManager`))
    (if _returnvalue
      (bind _returnvalue_2 (`EOSManager.ShutdownEOS` _activeeosmanager))
      (`KismetSystemLibrary.PrintString` (`KismetStringLibrary.Concat_StrStr` "Shutdown Success?: " (`|GetEnumeratorNameAsString` _returnvalue_2)) true true (struct :`G` 0.66 :`B` 1.0 :`A` 1.0) 10.0))))

(event `InputAction|InitMetric`
  (params (Key :type "Key Structure"))
  ;[1 1 1] Initialize the Metric.
  (:`Released`
    (bind _returnvalue (`EOSManager.GetMetrics`))
    (bind _returnvalue_2 (`EOSMetrics.InitMetric` _returnvalue))
    (`KismetSystemLibrary.PrintString` (`KismetStringLibrary.Concat_StrStr` "Init Metric Success?: " (`KismetStringLibrary.Conv_BoolToString` _returnvalue_2)) true true (struct :`R` 1.0 :`G` 0.872746 :`A` 1.0) 10.0)))

(event `InputAction|BeginMetricSession`
  (params (Key :type "Key Structure"))
  ;[1 1 1] Start a Player Session (Display Name is mandatory!)
  (:`Released`
    (bind _returnvalue (`EOSManager.GetMetrics`))
    (bind _returnvalue_2 (`EOSMetrics.BeginPlayerSession` _returnvalue "Test" "SAT_External" "ICT_MouseKeyboard"))
    (`KismetSystemLibrary.PrintString` (`KismetStringLibrary.Concat_StrStr` "Begin Player Session?: " (`KismetStringLibrary.Conv_BoolToString` _returnvalue_2)) true true (struct :`R` 0.039068 :`G` 0.359375 :`A` 1.0) 10.0)))

(event `InputAction|EndMetricSession`
  (params (Key :type "Key Structure"))
  ;[1 1 1] End a Player Session (Display Name should match the one used in Begin)
  (:`Released`
    (bind _returnvalue (`EOSManager.GetMetrics`))
    (bind _returnvalue_2 (`EOSMetrics.EndPlayerSession` _returnvalue "Test"))
    (`KismetSystemLibrary.PrintString` (`KismetStringLibrary.Concat_StrStr` "End Player Session?: " (`KismetStringLibrary.Conv_BoolToString` _returnvalue_2)) true true (struct :`R` 0.039068 :`G` 0.359375 :`A` 1.0) 10.0)))

(event `InputAction|Login`
  (params (Key :type "Key Structure"))
  ;[1 1 1] Basic handling of User Login/Logout Attempts. NOTE: You will need to be published on the Epic Store for this to work!
  (:`Released`
    (`KismetSystemLibrary.PrintString` "Login/Logout requires your project to be on EGS. There are also additional required C++ changes that would need to be made to get this to work." true true (struct :`R` 1.0 :`A` 1.0) 10.0 :!label _label)))

(event `LoggedIn`
  ;[1 1 1] Basic handling of User Login/Logout Attempts. NOTE: You will need to be published on the Epic Store for this to work!
  (`KismetSystemLibrary.PrintString` "Login Successful!" true true (struct :`G` 1.0 :`A` 1.0) 5.0))

(event `LoggedOut`
  ;[1 1 1] Basic handling of User Login/Logout Attempts. NOTE: You will need to be published on the Epic Store for this to work!
  (`KismetSystemLibrary.PrintString` "Logout Successful!" true true (struct :`G` 1.0 :`A` 1.0) 5.0))

(event `LoginFail`
  ;[1 1 1] Basic handling of User Login/Logout Attempts. NOTE: You will need to be published on the Epic Store for this to work!
  (`KismetSystemLibrary.PrintString` "Login FAILED!" true true (struct :`R` 1.0 :`A` 1.0) 5.0))

(event `RequiresMFA`
  ;[1 1 1] Basic handling of User Login/Logout Attempts. NOTE: You will need to be published on the Epic Store for this to work!
  (`KismetSystemLibrary.PrintString` "Login Requires MFA!" true true (struct :`R` 1.0 :`G` 0.198145 :`A` 1.0) 5.0))

(event `InputAction|Logout`
  (params (Key :type "Key Structure"))
  ;[1 1 1] Basic handling of User Login/Logout Attempts. NOTE: You will need to be published on the Epic Store for this to work!
  (:`Released`
    (goto _label)))

(fn `UserConstructionScript`)